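; Game mode for a multiplayer match that drives the Ready, Play and End phases through BP_GameState.
; On BeginPlay it binds to the game state's change and elapsed-time dispatchers and enters Ready, switching to Play after a few seconds.
; BindPlayerStates hooks a player state's GameOver dispatcher, but nothing here calls it.
; Game over calls UpdateWinner on every BP_MultiPlayerState, then sets End.
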(event `self.ReceiveBeginPlay`
  (`self.BindGameState`))

(fn `BindGameState`
  (bind _asbp_game_state (cast `/Game/MultiGame/BP_GameState` (`GameplayStatics.GetGameState`)))
  (add `/Game/MultiGame/BP_GameState.EventDispatcher_ChangeGameState` _asbp_game_state (`|CreateDelegate` :!event `EventChangeGameState`))
  (add `/Game/MultiGame/BP_GameState.EventDispatcher_TotalDeltaSec` _asbp_game_state (`|CreateDelegate` :!event `EventTotalDeltaSeconds`))
  (`/Game/MultiGame/BP_GameState.ChangeGameState` _asbp_game_state "NewEnumerator1"))

(fn `BindPlayerStates`
  (params (PlayerState :type "/Game/MultiGame/BP_MultiPlayerState Object Reference"))
  (add `/Game/MultiGame/BP_MultiPlayerState.EventDispatcher_GameOver` PlayerState (`|CreateDelegate` :!event `EventGameOver`)))

(fn `EventChangeGameState`
  (params (GameState :type "/Game/MultiGame/EN_GameState Enum" :default "NewEnumerator0"))
  (bind _output_get (set `self.Game State` GameState))
  (`KismetSystemLibrary.PrintString` (`KismetStringLibrary.Concat_StrStr` "Current GameState: " (`|GetEnumeratorNameAsString` _output_get)) true true (struct :`G` 0.66 :`B` 1.0 :`A` 1.0) 20.0))

(fn `EventGameOver`
  (`KismetSystemLibrary.PrintString` "GameOver")
  (`|ExecutionSequence`
    (:`then_0`
      (bind _outactors (`GameplayStatics.GetAllActorsOfClass` "/Game/MultiGame/BP_MultiPlayerState.BP_MultiPlayerState_C"))
      (for _array_element _outactors
        (`/Game/MultiGame/BP_MultiPlayerState.UpdateWinner` _array_element)))
    (:`then_1`
      (bind _asbp_game_state (cast `/Game/MultiGame/BP_GameState` (`GameplayStatics.GetGameState`)))
      (`/Game/MultiGame/BP_GameState.ChangeGameState` _asbp_game_state "NewEnumerator3"))))

(fn `EventTotalDeltaSeconds`
  (params (TotalDeltaSec :type "Float (double-precision)"))
  (switch `/Game/MultiGame/EN_GameState` (`self.Game State`)
    (:`NewEnumerator1`
      (if (> TotalDeltaSec 6.0)
        (bind _asbp_game_state (cast `/Game/MultiGame/BP_GameState` (`GameplayStatics.GetGameState`)))
        (`/Game/MultiGame/BP_GameState.ChangeGameState` _asbp_game_state "NewEnumerator2")))))

(fn `UserConstructionScript`)