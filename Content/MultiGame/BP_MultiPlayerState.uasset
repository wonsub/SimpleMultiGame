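; Multiplayer PlayerState that tracks a player's item count and win result in an item-collection game.
; On BeginPlay it registers with BP_MultiGameMode; AddCount increments the count up to a cap and fires a GameOver dispatcher on reaching it.
; UpdateWinner sets the IsWin enum, and RepNotifies on ItemCount and IsWin broadcast changes through dispatchers.
; EventGameOver is empty, with its HUD and pause logic left unconnected.
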(event `self.ReceiveBeginPlay`
  (bind _asbp_multi_game_mode (cast `/Game/MultiGame/BP_MultiGameMode` (`GameplayStatics.GetGameMode`)))
  (`/Game/MultiGame/BP_MultiGameMode.BindPlayerStates` _asbp_multi_game_mode self))

(fn `AddCount`
  (params (NewParam :type "Actor Object Reference"))
  (set `self.ItemCount` (`KismetMathLibrary.Clamp` (+ (`self.ItemCount`) 1) 0 10))
  (if (`self.IsWinner`)
    (`self.EventDispatcher_GameOver`)))

(fn `EventGameOver`)

(fn `IsWinner`
  (returns (IsWInner :type Boolean))
  (if (>= (`self.ItemCount`) 10)
    (return true)
    (else
      (return false))))

(fn `OnRep_IsWin`
  (`self.EventDispatcher_IsWin` (`self.IsWin`)))

(fn `OnRep_ItemCount`
  (`self.EventDispatcher_UpdateItemCount` (`self.ItemCount`)))

(fn `UpdateCountUI`
  (params (ItemCount :type Integer))
  (`/Game/MultiGame/HudWidget.UpdateItemCount` (`self.HudWidget`) ItemCount))

(fn `UpdateWinner`
  (if (>= (`self.ItemCount`) 10)
    (set `self.IsWin` "NewEnumerator1")
    (else
      (set `self.IsWin` "NewEnumerator2"))))

(fn `UserConstructionScript`)