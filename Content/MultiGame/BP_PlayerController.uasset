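; Player controller for a multiplayer game mode, built to gate character movement on game state changes.
; UpdateGameState sets the possessed BP_MultiCharacter to walking on the Play state; if the pawn cast fails, it schedules itself by a short function-name timer.
; BeginPlay is empty: the logic that disables movement and binds to BP_GameState's change-state dispatcher is disconnected and never runs.
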(event `self.ReceiveBeginPlay`)

(fn `UpdateGameState`
  (params (GameState :type "/Game/MultiGame/EN_GameState Enum" :default "NewEnumerator0"))
  (bind _asbp_multi_character (cast `/Game/MultiGame/BP_MultiCharacter` (`self.K2_GetPawn`))
    (:`then`
      (switch `/Game/MultiGame/EN_GameState` GameState
        (:`NewEnumerator2`
          (`CharacterMovementComponent.SetMovementMode` (`Character.CharacterMovement` _asbp_multi_character) "MOVE_Walking" 0))))
    (:`CastFailed`
      (`KismetSystemLibrary.K2_SetTimer` null "UpdateGameState" 0.01))))

(fn `UserConstructionScript`)